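; Game mode for LittleAlchemist that can build a map from a grid of randomly chosen chunk actors.
; AddChunk loops over the X by Y chunk count, advancing a row counter and spawning at tile-size spacing, with columns landing on negative X.
; SelectRandomClassType picks evenly between two minor chunk classes for each cell.
; Nothing in this graph calls AddChunk, and it prints the row counter on every spawn.
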(fn `AddChunk`
  (bind _defaulttilesize (`self.DefaultTileSize`))
  (bind _transformyvalue (`self.TransformYValue`))
  (for _index (range (* (`self.MapXChunkCount`) (`self.MapYChunkCount`)))
    (if (== (mod _index (`self.MapXChunkCount`)) 0)
      (`/Engine/EditorBlueprintResources/StandardMacros.IncrementInt` (`self.TransformYValue`)
        (:`  `
          _)))
    (bind _newparam (`self.SelectRandomClassType`))
    (`KismetSystemLibrary.PrintString` (`KismetStringLibrary.Conv_DoubleToString` (`KismetMathLibrary.Conv_IntToDouble` _transformyvalue)))
    (`|SpawnActorFromClass` _newparam (`KismetMathLibrary.MakeTransform` (`KismetMathLibrary.MakeVector` (`KismetMathLibrary.Conv_IntToDouble` (* (- _index (* _transformyvalue (`self.MapXChunkCount`))) _defaulttilesize)) (`KismetMathLibrary.Conv_IntToDouble` (* (- (`self.TransformYValue`) 1) _defaulttilesize)))) "Undefined" "OverrideRootScale" null null)))

(fn `SelectRandomClassType`
  (returns (NewParam :type "/Game/LittleAlchemistGame/Blueprints/LevelGeneration/Chunks/ConstructionChunks/Prototype/Chunk Class Reference"))
  (switch `int` (`KismetMathLibrary.RandomInteger` 2)
    (:`Default`
      _)
    (:`0`
      _)
    (:`1`
      (return "/Game/LittleAlchemistGame/Blueprints/LevelGeneration/Chunks/ConstructionChunks/Prototype/MinorChunk2.MinorChunk2_C")))
  (return "/Game/LittleAlchemistGame/Blueprints/LevelGeneration/Chunks/ConstructionChunks/Prototype/MinorChunk1.MinorChunk1_C"))

(fn `UserConstructionScript`)
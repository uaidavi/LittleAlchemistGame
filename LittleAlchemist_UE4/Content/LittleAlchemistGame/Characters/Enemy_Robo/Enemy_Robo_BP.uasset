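; Robo enemy Blueprint whose graph only drives proximity music, with "ChefeVolume" suggesting a boss layer.
; Any overlap entering or leaving MusicSphere switches the track on LittleAlchemistGM and sets old and new volumes for fading in or out.
; A shared timeline feeds the blend alpha to the game mode's AddRemoveEnemySound each update.
; Both events call Play rather than PlayFromStart, so the timeline is never explicitly rewound.
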(event `self.MusicSphere.OnComponentBeginOverlap`
  (params (OverlappedComponent :type "PrimitiveComponent Object Reference") (OtherActor :type "Actor Object Reference") (OtherComp :type "PrimitiveComponent Object Reference") (OtherBodyIndex :type Integer) (bFromSweep :type Boolean) (SweepResult :type "HitResult Structure (by ref)"))
  (bind _aslittle_alchemist_gm (cast `/Game/LittleAlchemistGame/LittleAlchemistGM` (`GameplayStatics.GetGameMode`))
    (:`then`
      (`/Game/LittleAlchemistGame/LittleAlchemistGM.ChangeTrack` _aslittle_alchemist_gm 1.0)
      (set `self.OldVolume` 0.0)
      (set `self.NewVolume` 1.0)
      (bind (_direction _newtrack_0) (`Timeline|Timeline_0` :!label _label)
        (:`Update`
          (bind _aslittle_alchemist_gm_2 (cast `/Game/LittleAlchemistGame/LittleAlchemistGM` (`GameplayStatics.GetGameMode`))
            (:`then`
              (`/Game/LittleAlchemistGame/LittleAlchemistGM.AddRemoveEnemySound` _aslittle_alchemist_gm_2 (`self.OldVolume`) (`self.NewVolume`) _newtrack_0 "ChefeVolume"))
            (:`CastFailed`
              (`KismetSystemLibrary.PrintString` "Hello"))))))
    (:`CastFailed`
      (`KismetSystemLibrary.PrintString` "lulno" :!label _label_2))))

(event `self.MusicSphere.OnComponentEndOverlap`
  (params (OverlappedComponent :type "PrimitiveComponent Object Reference") (OtherActor :type "Actor Object Reference") (OtherComp :type "PrimitiveComponent Object Reference") (OtherBodyIndex :type Integer))
  (bind _aslittle_alchemist_gm (cast `/Game/LittleAlchemistGame/LittleAlchemistGM` (`GameplayStatics.GetGameMode`))
    (:`then`
      (`/Game/LittleAlchemistGame/LittleAlchemistGM.ChangeTrack` _aslittle_alchemist_gm 0.0)
      (set `self.OldVolume` 1.0)
      (set `self.NewVolume` 0.0)
      (goto _label))
    (:`CastFailed`
      (goto _label_2))))

(fn `UserConstructionScript`)
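; Generic AI enemy character with a health bar widget that takes damage, attacks the player and dies.
; Damage is reported to AI perception, and death decrements the owning chunk's KillEnemiesEvent count, completing the event at zero.
; Attacks freeze movement and flag GenEnemyAnimBP, then a separate apply-damage event hurts the player if inside AtkColl and restores walking.
; A ForceSight overlap writes the overlapping actor and its distance straight to the GenEnemyAI blackboard.
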(event `self.Box.OnComponentBeginOverlap`
  (params (OverlappedComponent :type "PrimitiveComponent Object Reference") (OtherActor :type "Actor Object Reference") (OtherComp :type "PrimitiveComponent Object Reference") (OtherBodyIndex :type Integer) (bFromSweep :type Boolean) (SweepResult :type "HitResult Structure (by ref)")))

(event `self.Box.OnComponentEndOverlap`
  (params (OverlappedComponent :type "PrimitiveComponent Object Reference") (OtherActor :type "Actor Object Reference") (OtherComp :type "PrimitiveComponent Object Reference") (OtherBodyIndex :type Integer)))

(event `self.ReceiveBeginPlay`
  (bind _returnvalue (`|CreateWidget` "/Game/LittleAlchemistGame/Characters/GenericEnemy/EnemyHealthBar.EnemyHealthBar_C"))
  (bind _output_get (set `self.WDG_HealthBar` _returnvalue))
  (`WidgetComponent.SetWidget` (`self.HealthBar1`) _output_get)
  (set `/Game/LittleAlchemistGame/Characters/GenericEnemy/EnemyHealthBar.EnemyRef` self (`self.WDG_HealthBar`))
  (`self.SpawnDefaultController`))

(event `AmEnemy`
  (`KismetSystemLibrary.PrintString` "AmEnemy" true true (struct :`R` 1.0 :`B` 0.023671 :`A` 1.0) 10.0))

(event `self.ReceiveAnyDamage`
  (params (Damage :type "Float (single-precision)") (DamageType :type "DamageType Object Reference") (InstigatedBy :type "Controller Object Reference") (DamageCauser :type "Actor Object Reference"))
  (bind _returnvalue (`self.K2_GetActorLocation` self))
  (`AISense_Damage.ReportDamageEvent` self (`Controller.K2_GetPawn` (`GameplayStatics.GetPlayerController` 0)) Damage _returnvalue _returnvalue)
  (`KismetSystemLibrary.PrintString` "DamageReceived" true true (struct :`R` 1.0 :`B` 0.023671 :`A` 1.0) 10.0)
  (bind _output_get (set `self.CurHealth` (- (`self.CurHealth`) (`KismetMathLibrary.FTrunc` Damage))))
  (if (<= _output_get 0)
    (`self.EnemyDeath`)))

(event `EnemyDeath`
  (`KismetSystemLibrary.Delay` 0.2)
  (`self.K2_DestroyActor`)
  (bind _askill_enemies_event (cast `/Game/LittleAlchemistGame/Gameplay/KillEnemiesEvent` (`/Game/LittleAlchemistGame/LevelGeneration/Chunks/ConstructionChunks/Prototype/Chunk.ChunkEvent` (`self.OwningChunk`))))
  (bind _result (`/Engine/EditorBlueprintResources/StandardMacros.DecrementInt` (`/Game/LittleAlchemistGame/Gameplay/KillEnemiesEvent.EnemyCount` _askill_enemies_event))
    (:`  `
      (if (<= _result 0)
        (set `/Game/LittleAlchemistGame/Gameplay/BaseChunkEvent.IsCompleted` true _askill_enemies_event)))))

(event `/Game/LittleAlchemistGame/Characters/GenericEnemy/EnemyEvents.SetAlertState`
  (params (EnemyAlertState :type "/Game/LittleAlchemistGame/Characters/GenericEnemy/EnumEnemyState Enum" :default "NewEnumerator2"))
  (set `self.AlertState` EnemyAlertState))

(event `self.ReceiveTick`
  (params (DeltaSeconds :type "Float (single-precision)")))

(event `/Game/LittleAlchemistGame/Characters/GenericEnemy/EnemyEvents.Attack`
  (params (AttackDamage :type Integer) (AttackID :type Integer))
  (bind _output_get (set `self.IsAttacking` true))
  (bind _asgen_enemy_anim_bp (cast `/Game/LittleAlchemistGame/Characters/GenericEnemy/GenEnemyAnimBP` (`SkeletalMeshComponent.GetAnimInstance` (`self.Mesh`))))
  (set `/Game/LittleAlchemistGame/Characters/GenericEnemy/GenEnemyAnimBP.IsAttacking` _output_get _asgen_enemy_anim_bp)
  (cast `/Game/LittleAlchemistGame/Characters/Main_Cacau/Control/Cacau_CharBP` (`Controller.K2_GetPawn` (`GameplayStatics.GetPlayerController` 0)))
  (switch `int` AttackID
    (:`Default`
      _)
    (:`0`
      _))
  (`CharacterMovementComponent.DisableMovement` (`self.CharacterMovement`))
  (`KismetSystemLibrary.PrintString` "TryAttacj"))

(event `/Game/LittleAlchemistGame/Characters/GenericEnemy/EnemyEvents.AttackApplyDamage`
  (params (AttackID :type Integer))
  (bind _returnvalue (`Controller.K2_GetPawn` (`GameplayStatics.GetPlayerController` 0)))
  (`KismetSystemLibrary.PrintString` "Attack")
  (switch `int` AttackID
    (:`Default`
      _)
    (:`0`
      _))
  (`KismetSystemLibrary.PrintString` "Hello")
  (if (`PrimitiveComponent.IsOverlappingActor` (`self.AtkColl`) _returnvalue)
    (`GameplayStatics.ApplyDamage` _returnvalue (`KismetMathLibrary.Conv_IntToDouble` (stale `/Game/LittleAlchemistGame/Characters/GenericEnemy/EnemyEvents.Attack` AttackDamage))))
  (`CharacterMovementComponent.SetMovementMode` (`self.CharacterMovement`) "MOVE_Walking" 0)
  (bind _output_get (set `self.IsAttacking` false))
  (bind _asgen_enemy_anim_bp (cast `/Game/LittleAlchemistGame/Characters/GenericEnemy/GenEnemyAnimBP` (`SkeletalMeshComponent.GetAnimInstance` (`self.Mesh`))))
  (set `/Game/LittleAlchemistGame/Characters/GenericEnemy/GenEnemyAnimBP.IsAttacking` _output_get _asgen_enemy_anim_bp))

(event `self.ForceSight.OnComponentBeginOverlap`
  (params (OverlappedComponent :type "PrimitiveComponent Object Reference") (OtherActor :type "Actor Object Reference") (OtherComp :type "PrimitiveComponent Object Reference") (OtherBodyIndex :type Integer) (bFromSweep :type Boolean) (SweepResult :type "HitResult Structure (by ref)"))
  (bind _asgen_enemy_ai (cast `/Game/LittleAlchemistGame/Characters/GenericEnemy/GenEnemyAI` (`self.GetController`)))
  (bind _returnvalue (`AIBlueprintHelperLibrary.GetBlackboard` _asgen_enemy_ai))
  (`BlackboardComponent.SetValueAsObject` _returnvalue "TargetActor" OtherActor)
  (`BlackboardComponent.SetValueAsFloat` _returnvalue "TargetDistance" (`KismetMathLibrary.Vector_Distance` (`self.K2_GetActorLocation` self) (`self.K2_GetActorLocation` OtherActor))))

(fn `Attack_1`
  (params (Damage :type Integer) (cacau :type "/Game/LittleAlchemistGame/Characters/Main_Cacau/Control/Cacau_CharBP Object Reference"))
  (`SkeletalMeshComponent.PlayAnimation` (`self.Mesh`) "/Game/LittleAlchemistGame/Characters/Enemy_Jacare/Jacare_Attack.Jacare_Attack" false)
  (`GameplayStatics.ApplyDamage` cacau (`KismetMathLibrary.Conv_IntToDouble` Damage))
  (return))

(fn `UserConstructionScript`)